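; Enemy shooter character Blueprint that shows visual feedback whenever it takes damage.
; AnyDamage predicts the new health fraction by subtracting damage over max health from the current percentage and passes it to the health bar widget.
; It also plays the damage amount on a text widget and triggers a hitmarker on the first player controller's HUD, without checking who dealt the damage.
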(event `self.ReceiveAnyDamage`
  (params (Damage :type "Float (single-precision)") (DamageType :type "DamageType Object Reference") (InstigatedBy :type "Controller Object Reference") (DamageCauser :type "Actor Object Reference"))
  (`|ExecutionSequence`
    (:`then_0`
      ;[1 1 1] calc helth bar fill percent
      (bind _returnvalue (`self.GetMaxHealth`))
      (bind _returnvalue_2 (`self.GetHealthProcentage`))
      ;[1 1 1] Play health bar
      (bind _aswbp_health (cast `/Game/IN_Blueprints/Widgets/WBP_Health` (`WidgetComponent.GetUserWidgetObject` (`self.HealthBar`))))
      (`/Game/IN_Blueprints/Widgets/WBP_Health.ShowHealthBar` _aswbp_health (- _returnvalue_2 (/ Damage _returnvalue))))
    (:`then_1`
      ;[1 1 1] Play damage
      (bind _aswbp_damage (cast `/Game/IN_Blueprints/Widgets/WBP_Damage` (`WidgetComponent.GetUserWidgetObject` (`self.DamageText`))))
      (`/Game/IN_Blueprints/Widgets/WBP_Damage.PlayDamageText` _aswbp_damage Damage))
    (:`then_2`
      (bind _asbp_western_shooter_controller (cast `/Game/IN_Blueprints/BP_WesternShooterController` (`GameplayStatics.GetPlayerController` 0)))
      (bind _aswbp_hud (cast `/Game/IN_Blueprints/Widgets/WBP_HUD` (`WesternShooterPlayerController.GetHUDWidget` _asbp_western_shooter_controller)))
      (`/Game/IN_Blueprints/Widgets/WBP_HUD.PlayHitmarker` _aswbp_hud))))

(fn `UserConstructionScript`
  (`parent.UserConstructionScript`))